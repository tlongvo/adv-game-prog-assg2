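; Enemy character Blueprint for a networked AI that fires a gun held in a child actor.
; Fire, expected to run on the server, waits for the gun's fire rate, shoots, rotates the enemy to the aim direction and multicasts.
; Simulated proxies replay the shot and rotation using the server's spread direction.
; Spread multiplies the aim component-wise by a random unit vector scaled by TargetAccuracyOffset, rather than adding an offset.
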(event Custom|MulticastFire
  (params (Fire%20Direction :type Vector) (Rotation :type Rotator))
  ;[1 1 1] Fire Event that occurs on the Server (Authority Role of AI). Thus Only need to multicast this behaviour down to the Players who see AI as Simulated Proxies
  (if (Utilities|Enum|Equal(Enum) (Networking|GetLocalRole) "ROLE_SimulatedProxy")
    (bind _asgun_blueprint (Utilities|Casting|CastToGunBlueprint (Variables|/Script/Engine.ChildActorComponent|GetChildActor (Variables|Default|GetGun))))
    (Default|Fire _asgun_blueprint Fire%20Direction)
    (Transformation|SetActorRotation Rotation)))

(event EventBeginPlay)

(event Collision|EventActorBeginOverlap
  (params (OtherActor :type Actor%20Object%20Reference)))

(event EventTick
  (params (DeltaSeconds :type Float%20%28single-precision%29)))

(event EventFire
  (params (FireDirection :type Vector :default "0, 0, 0"))
  (bind _returnvalue (Math|Conversions|RotationFromXVector FireDirection))
  ;[1 1 1] Fire Event that occurs on the Server (Authority Role of AI). Thus Only need to multicast this behaviour down to the Players who see AI as Simulated Proxies
  (bind _asgun_blueprint (Utilities|Casting|CastToGunBlueprint (Variables|/Script/Engine.ChildActorComponent|GetChildActor (Variables|Default|GetGun))))
  (Utilities|FlowControl|Delay (Variables|/Game/Blueprints/GunBlueprint.GunBlueprint_C|GetFireRate _asgun_blueprint))
  (bind _newpath (CallFunction|CreateMoreBulletSpread FireDirection))
  (Default|Fire _asgun_blueprint _newpath)
  (Transformation|SetActorRotation _returnvalue)
  (CallFunction|MulticastFire _newpath _returnvalue))

(fn ConstructionScript)

(fn CreateMoreBulletSpread
  (params (Direction :type Vector))
  (return (* (* (Math|Random|RandomUnitVector) (Variables|Default|GetTargetAccuracyOffset)) Direction)))