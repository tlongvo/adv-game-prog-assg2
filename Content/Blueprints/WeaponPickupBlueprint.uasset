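; Weapon pickup Blueprint that shows its rarity and passes its weapon stats to the gun of the actor that picks it up.
; On BeginPlay it calls OnGenerate, then sets the Gun material to match Common, Rare, Master or Legendary rarity.
; OnPickup casts the actor's child actors to GunBlueprint, overwrites the gun's stats, refills its magazine and destroys the pickup.
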(event EventBeginPlay
  (Class|WeaponPickup|OnGenerate)
  (if (Utilities|Enum|Equal(Enum) (Variables|Default|GetRarity) "LEGENDARY")
    (Rendering|Material|SetMaterial (Variables|Default|GetGun) 0 "/Game/Materials/WeaponRarityMaterials/LegendaryMaterial.LegendaryMaterial")
    (elif (Utilities|Enum|Equal(Enum) (Variables|Default|GetRarity) "MASTER")
      (Rendering|Material|SetMaterial (Variables|Default|GetGun) 0 "/Game/Materials/WeaponRarityMaterials/MasterMaterial.MasterMaterial")
      (elif (Utilities|Enum|Equal(Enum) (Variables|Default|GetRarity) "RARE")
        (Rendering|Material|SetMaterial (Variables|Default|GetGun) 0 "/Game/Materials/WeaponRarityMaterials/RareMaterial.RareMaterial")
        (elif (Utilities|Enum|Equal(Enum) (Variables|Default|GetRarity) "COMMON")
          (Rendering|Material|SetMaterial (Variables|Default|GetGun) 0 "/Game/Materials/WeaponRarityMaterials/CommonMaterial.CommonMaterial"))))))

(event Collision|EventActorBeginOverlap
  (params (OtherActor :type Actor%20Object%20Reference)))

(event EventTick
  (params (DeltaSeconds :type Float%20%28single-precision%29)))

(event EventOnPickup
  (params (ActorThatPickedUp :type Actor%20Object%20Reference))
  (for _array_element (Actor|GetComponentsByClass ActorThatPickedUp "/Script/Engine.ChildActorComponent")
    (bind _asgun_blueprint (Utilities|Casting|CastToGunBlueprint (Variables|/Script/Engine.ChildActorComponent|GetChildActor _array_element)))
    (Variables|/Game/Blueprints/GunBlueprint.GunBlueprint_C|SetMuzzleVelocity _asgun_blueprint (Variables|Default|GetMuzzleVelocity))
    (Variables|/Game/Blueprints/GunBlueprint.GunBlueprint_C|SetBulletDamage _asgun_blueprint (Variables|Default|GetBulletDamage))
    (bind _output_get (Variables|/Game/Blueprints/GunBlueprint.GunBlueprint_C|SetMagazineSize _asgun_blueprint (Variables|Default|GetMagazineSize)))
    (Variables|/Game/Blueprints/GunBlueprint.GunBlueprint_C|SetRoundsRemainingInMagazine _asgun_blueprint _output_get)
    (Variables|/Game/Blueprints/GunBlueprint.GunBlueprint_C|SetWeaponAccuracy _asgun_blueprint (Variables|Default|GetWeaponAccuracy))
    (Actor|DestroyActor)))

(fn ConstructionScript)