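; Replicated gun actor that handles firing, ammo and reloading for its parent character.
; Server-side Tick runs the fire-rate cooldown that re-enables CanFire while rounds remain.
; Fire traces predicted projectile paths with random spread, multiple for SHOT type, playing sound, player montage and impact effects, while the server damages HealthComponents and notifies hit enemies.
; RepNotifies on magazine variables refresh the locally controlled player's ammo HUD.
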(event EventBeginPlay
  (Variables|Default|SetRoundsRemainingInMagazine (Variables|Default|GetMagazineSize)))

(event Collision|EventActorBeginOverlap
  (params (OtherActor :type Actor%20Object%20Reference)))

(event EventTick
  (params (DeltaSeconds :type Float%20%28single-precision%29))
  (Networking|SwitchHasAuthority
    (:Authority
      (bind _output_get (Variables|Default|SetTimeTillNextShot (- (Variables|Default|GetTimeTillNextShot) DeltaSeconds)))
      (if (not (Variables|Default|GetbCanFire))
        (if (and (<= _output_get 0.0) (> (Variables|Default|GetRoundsRemainingInMagazine) 0))
          (Variables|Default|SetbCanFire true))))))

(fn ConstructionScript)

(fn Fire
  (params (LaunchDirection :type Vector))
  (bind _muzzleposition (Variables|Default|GetMuzzlePosition))
  (bind _returnvalue (Transformation|GetWorldLocation _muzzleposition))
  (if (Variables|Default|GetbCanFire)
    (Networking|SwitchHasAuthority
      (:Authority
        (Variables|Default|SetbCanFire (not (Variables|Default|GetbCanFire)))
        (Variables|Default|SetTimeTillNextShot (Variables|Default|GetFireRate)))
      (:Remote
        _))
    ;[1 1 1] Multishot Implementation
    (if (Utilities|Enum|Equal(Enum) (Variables|Default|GetWeaponFiringType) "MULTI_SHOT")
      (Variables|Default|SetShotCount 4)
      (else
        (Variables|Default|SetShotCount 0)))
    (for _index (range 0 (Variables|Default|GetShotCount))
      (bind _outhit (Class|GameplayStatics|BlueprintPredictProjectilePathbyTraceChannel _returnvalue (* (Math|Vector|Normalize (+ (Math|Random|RandomUnitVector) (* LaunchDirection (Variables|Default|GetWeaponAccuracy)))) (Variables|Default|GetMuzzleVelocity)) true 1.0 "ECC_WorldDynamic" false 0 "ForDuration" 4.0))
      (Variables|Default|SetRoundsRemainingInMagazine (- (Variables|Default|GetRoundsRemainingInMagazine) 1))
      (Audio|PlaySoundatLocation "/Game/Assets/Audio/FirstPersonTemplateWeaponFire02.FirstPersonTemplateWeaponFire02" _returnvalue "0, 0, 0" 1.0 1.0 0.0 0 0 0)
      (bind _asplayer_character_blueprint (Utilities|Casting|CastToPlayerCharacterBlueprint (Actor|GetParentActor))
        (:then
          (Animation|Montage|MontagePlay (Components|SkeletalMesh|GetAnimInstance (Variables|/Game/Blueprints/PlayerCharacterBlueprint.PlayerCharacterBlueprint_C|GetArms _asplayer_character_blueprint)) "/Game/Assets/Arms/Animations/FirstPersonFire_Montage.FirstPersonFire_Montage" 1.0 "MontageLength" 0.0 true)
          (if (Utilities|IsValid (.HitActor (Collision|BreakHitResult _outhit)))
            (if (Utilities|IsValid (Actor|GetComponentbyClass (.HitActor (Collision|BreakHitResult _outhit)) "/Script/AdvGamesProgramming.HealthComponent"))
              (Effects|SpawnEmitteratLocation "/Game/ParticleEffects/Gun/BulletImpactOnCharacter.BulletImpactOnCharacter" (.Location (Collision|BreakHitResult _outhit)) (Math|Rotator|MakeRotfromZ (.Normal (Collision|BreakHitResult _outhit))))
              (else
                (Effects|SpawnEmitteratLocation "/Game/ParticleEffects/Gun/BulletImpact.BulletImpact" (.Location (Collision|BreakHitResult _outhit)))))
            (if (and (Utilities|IsValid (.HitActor (Collision|BreakHitResult _outhit))) (Networking|IsServer)) :!label _label
              (if (Utilities|IsValid (Actor|GetComponentbyClass (.HitActor (Collision|BreakHitResult _outhit)) "/Script/AdvGamesProgramming.HealthComponent"))
                (Class|HealthComponent|OnTakeDamage (Actor|GetComponentbyClass (.HitActor (Collision|BreakHitResult _outhit)) "/Script/AdvGamesProgramming.HealthComponent") (Variables|Default|GetBulletDamage))
                (Development|PrintString (Utilities|String|ToString(Float) (Variables|/Script/AdvGamesProgramming.HealthComponent|GetCurrentHealth (Actor|GetComponentbyClass (.HitActor (Collision|BreakHitResult _outhit)) "/Script/AdvGamesProgramming.HealthComponent"))) true false)
                (bind _asenemy_character (Utilities|Casting|CastToEnemyCharacter (Components|GetOwner (Variables|/Script/Engine.Actor|GetRootComponent (.HitActor (Collision|BreakHitResult _outhit))))))
                (if (Utilities|IsValid _asenemy_character)
                  (Development|PrintString "HIT ENEMY")
                  (Class|EnemyCharacter|OnHit _asenemy_character)
                  (Utilities|Casting|CastToUE4ASP_HeroTPP_AnimBlueprint (Components|SkeletalMesh|GetAnimInstance (Variables|/Script/Engine.Character|GetMesh _asenemy_character))))
                (else
                  (Development|PrintString "Did not hit actor with health component" true false))))))
        (:CastFailed
          (goto _label))))))

(fn Reload
  (Variables|Default|SetRoundsRemainingInMagazine (Variables|Default|GetMagazineSize)))

(fn UpdateAmmoHUD
  (bind _asplayer_character_blueprint (Utilities|Casting|CastToPlayerCharacterBlueprint (Actor|GetParentActor)))
  (if (Pawn|IsLocallyControlled _asplayer_character_blueprint)
    (bind _asplayer_controller (Utilities|Casting|CastToPlayerController (Pawn|GetController _asplayer_character_blueprint)))
    (bind _asplayer_hud (Utilities|Casting|CastToPlayerHUD (HUD|GetHUD _asplayer_controller)))
    (Class|PlayerHUD|SetAmmoText _asplayer_hud (Variables|Default|GetRoundsRemainingInMagazine) (Variables|Default|GetMagazineSize))))

(fn OnRepRoundsRemaininginMagazine
  (CallFunction|UpdateAmmoHUD))

(fn OnRepMagazineSize
  (CallFunction|UpdateAmmoHUD))